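; BP_PCG_NiagaraParam is a Blueprint that regenerates its PCG component based on changes in a tracked float value.
; SetVal copies Val into CurrentVal, and SetPrev stores it as PrevVal.
; ForceGeneratePCG force-generates the PCG when CurrentVal is greater than or equal to PrevVal, skipping decreases.
; The event graph does no work, as its ForceGeneratePCG call is disconnected, and no Niagara access appears in these graphs.
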(event EventBeginPlay)

(event Collision|EventActorBeginOverlap
  (params (OtherActor :type Actor%20Object%20Reference)))

(event EventTick
  (params (DeltaSeconds :type Float%20%28single-precision%29)))

(fn ConstructionScript)

(fn SetVal
  (Variables|Internal|SetCurrentVal (Variables|Default|GetVal)))

(fn ForceGeneratePCG
  (Math|Float|CompareFloat (Variables|Internal|GetCurrentVal) (Variables|Internal|GetPrevVal)
    (:>
      _)
    (:==
      _))
  (PCG|Generate (Variables|Default|GetPCG) true))

(fn SetPrev
  (Variables|Internal|SetPrevVal (Variables|Internal|GetCurrentVal)))